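; BP_masterPieces is a breakable-piece actor that, judging by its name and folder, serves as the base for debris fragments.
; On BeginPlay it applies outer and inner materials and a mesh from its variables to its static mesh component, then enables physics.
; It launches the piece with a random, mass-independent velocity impulse that is always positive on each axis.
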(event EventBeginPlay
  (bind _staticmesh (Variables|Default|GetStaticMesh))
  (Rendering|Material|SetMaterial _staticmesh 0 (Variables|Default|GetobjectMaterial))
  (Rendering|Material|SetMaterial _staticmesh 1 (Variables|Default|GetobjectInnerMaterial))
  (Components|StaticMesh|SetStaticMesh _staticmesh (Variables|Default|GetobjectMesh))
  (Physics|SetSimulatePhysics _staticmesh true)
  (Class|PrimitiveComponent|WakeAllRigidBodies _staticmesh)
  (Physics|AddImpulse (Variables|Default|GetStaticMesh) (Math|Vector|MakeVector (Math|Random|RandomFloatinRange 75.0 2.5e+02) (Math|Random|RandomFloatinRange 75.0 2.5e+02) (Math|Random|RandomFloatinRange 75.0 2.5e+02)) "None" true))

(fn ConstructionScript)