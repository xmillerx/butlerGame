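; BP_breakableSpawner scatters randomly chosen breakable objects inside a box volume, starting at BeginPlay.
; A looping timer, whose period is a random interval rolled once and divided by the target count, calls spawnObject.
; Each tick picks a BP_breakableMaster class from the candidate list and spawns it at a random point within SpawnExtent.
; The timer clears once the spawn counter exceeds the target, so one extra object spawns.
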(event Custom|startSpawning
  (bind _returnvalue (Utilities|Time|SetTimerbyFunctionName 0 "spawnObject" (/ (Math|Random|RandomFloatinRange (Variables|Default|GetintervalMin) (Variables|Default|GetintervalMax)) (Math|Conversions|ToFloat(Integer) (Variables|Default|GettotalObjectsToSpawn))) true))
  (Variables|Default|SetspawnObject_timer _returnvalue))

(event Custom|spawnObject
  (bind _spawnextent (Variables|Default|GetSpawnExtent))
  (CallFunction|RandomizeSpawnedObject)
  (Game|SpawnActorfromClass (Variables|Default|GetbreakableObjectClass) (Math|Transform|MakeTransform (Math|Random|RandomPointinBoundingBox (Transformation|GetWorldLocation _spawnextent) (Variables|/Script/Engine.BoxComponent|GetBoxExtent _spawnextent)) "0, 0, 0" "1,1,1") "Undefined" 0 0)
  (Variables|Default|SetspawnedObjects (+ (Variables|Default|GetspawnedObjects) 1))
  (if (> (Variables|Default|GetspawnedObjects) (Variables|Default|GettotalObjectsToSpawn))
    (Utilities|Time|ClearandInvalidateTimerbyHandle (Variables|Default|GetspawnObject_timer))))

(event EventBeginPlay
  (CallFunction|StartSpawning))

(fn ConstructionScript)

(fn RandomizeSpawnedObject
  (bind _possiblebreakablespawninglist (Variables|Default|GetpossibleBreakableSpawningList))
  (Variables|Default|SetbreakableObjectClass (.AsBP%20Breakable%20Master (Utilities|Casting|CastToBP_breakableMasterClass (Utilities|Array|Get(acopy) _possiblebreakablespawninglist (Math|Random|RandomIntegerinRange 0 (- (Utilities|Array|Length _possiblebreakablespawninglist) 1)))))))