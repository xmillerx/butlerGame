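; Master Blueprint for breakable objects in the butler game, which shatter into pieces the first time their mesh registers a hit.
; Construction applies the configurable mesh, dynamic material, break effect and sounds.
; BeginPlay adds the difficulty-selected piece array's length to the game state's total.
; Break plays a sound, hides the mesh and spawns a BP_masterPieces actor per array entry; Swept only plays audio and KeepScore is empty.
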(event OnComponentHit(SM_displayObject)
  (params (HitComponent :type Primitive%20Component%20Object%20Reference) (OtherActor :type Actor%20Object%20Reference) (OtherComp :type Primitive%20Component%20Object%20Reference) (NormalImpulse :type Vector :default "0, 0, 0") (Hit :type Hit%20Result%20Structure%20%28by%20ref%29))
  (Utilities|FlowControl|DoOnce false
    (:Completed
      (CallFunction|Break))))

(event EventBeginPlay
  (Default|AddtoTotalPieces (.AsGS%20Butler%20Game (Utilities|Casting|CastToGS_butlerGame (Game|GetGameState))) (Utilities|Array|Length (Utilities|Select :Index (Math|Conversions|ToInteger(Byte) (Variables|Default|GetobjectDifficulty)) :Option%200 (Variables|Default|GeteasyArray) :Option%201 (Variables|Default|GetmediumArray) :Option%202 (Variables|Default|GethardArray)))))

(event Collision|EventActorBeginOverlap
  (params (OtherActor :type Actor%20Object%20Reference)))

(event EventTick
  (params (DeltaSeconds :type Float%20%28single-precision%29)))

(fn ConstructionScript
  (CallFunction|Ini))

(fn Ini
  (bind _sm_displayobject (Variables|Default|GetSM_displayObject))
  (Components|StaticMesh|SetStaticMesh _sm_displayobject (Variables|Default|GetobjectMesh))
  (bind _returnvalue (Rendering|Material|CreateDynamicMaterialInstance _sm_displayobject 0 (Variables|Default|GetobjectMaterial) :!class /Script/Engine.PrimitiveComponent))
  (Variables|Default|Setobject_DMI _returnvalue)
  (Effects|Components|ParticleSystem|SetTemplate (Variables|Default|GetPFX_break) (Variables|Default|GetobjectBreakFX))
  (Audio|Components|Audio|SetSound (Variables|Default|GetA_hit) (Variables|Default|GetobjectHitSound))
  (Audio|Components|Audio|SetSound (Variables|Default|GetA_break) (Variables|Default|GetobjectBreakSound))
  (Audio|Components|Audio|SetSound (Variables|Default|GetA_swept) (Variables|Default|GetobjectSweptSound))
  (Audio|Components|Audio|SetSound (Variables|Default|GetA_trashed) (Variables|Default|GetobjectTrashedSound)))

(fn Break
  (Components|Activation|Activate (Variables|Default|GetA_break) false)
  (Development|SetHiddeninGame (Variables|Default|GetSM_displayObject) true false)
  (CallFunction|SpawnPieces))

(fn Swept
  (Components|Activation|Activate (Variables|Default|GetA_swept) true))

(fn KeepScore)

(fn SpawnPieces
  (bind _easyarray (Variables|Default|GeteasyArray))
  (bind _objectdifficulty (Variables|Default|GetobjectDifficulty))
  (bind _mediumarray (Variables|Default|GetmediumArray))
  (bind _hardarray (Variables|Default|GethardArray))
  (bind _returnvalue (Math|Conversions|ToInteger(Byte) _objectdifficulty))
  (bind _returnvalue_2 (Utilities|Select :Index _returnvalue :Option%200 _easyarray :Option%201 _mediumarray :Option%202 _hardarray))
  (for _index (range 0 (- (Utilities|Array|Length _returnvalue_2) 1))
    (bind _returnvalue_3 (Game|SpawnActorfromClass "/Game/INFRASTRUCTURE/breakables/BP_masterPieces.BP_masterPieces_C" (Transformation|GetActorTransform) "Undefined" 0 (Utilities|Array|Get(acopy) _returnvalue_2 _index) (Rendering|Material|GetMaterial (Variables|Default|GetSM_displayObject) 0)))
    (Variables|/Game/INFRASTRUCTURE/breakables/BP_masterPieces.BP_masterPieces_C|SetobjectMesh (.AsBP%20Master%20Pieces (Utilities|Casting|CastToBP_masterPieces _returnvalue_3)) (Utilities|Array|Get(acopy) _returnvalue_2 _index))))