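; Actor component that fades the static mesh of its owning StaticMeshActor in or out through material opacity.
; BeginPlay creates and stores a dynamic material instance for each of the mesh's material slots.
; Every tick it moves a clamped fade value by FadeRate, down when Hidden and up otherwise, then writes it through FadeCurve to each instance's "opacity" parameter.
; ToggleHideMesh sets the Hidden state that drives the fade direction.
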(event EventBeginPlay
  (bind _asstatic_mesh_actor (Utilities|Casting|CastToStaticMeshActor (Components|GetOwner)))
  (bind _output_get (Variables|Default|SetparentMesh _asstatic_mesh_actor))
  (for (_array_element _array_index) (Rendering|Material|GetMaterials (Variables|/Script/Engine.StaticMeshActor|GetStaticMeshComponent _output_get))
    (bind _returnvalue (Rendering|Material|CreateDynamicMaterialInstance (Variables|/Script/Engine.StaticMeshActor|GetStaticMeshComponent _output_get) _array_index _array_element :!class /Script/Engine.PrimitiveComponent))
    (Utilities|Array|Add (Variables|Default|GetFadeMatMID) _returnvalue)))

(event EventTick
  (params (DeltaSeconds :type Float%20%28single-precision%29))
  (Variables|Default|SetDeltaTime DeltaSeconds)
  (Utilities|IsValid (Variables|Default|GetparentMesh)
    (:Is%20Valid
      (if (Variables|Default|GetHidden)
        (Variables|Default|SetCurrentFade (Math|Float|Clamp(Float) (- (Variables|Default|GetCurrentFade) (* (Variables|Default|GetDeltaTime) (Variables|Default|GetFadeRate)))))
        (else
          (Variables|Default|SetCurrentFade (Math|Float|Clamp(Float) (+ (Variables|Default|GetCurrentFade) (* (Variables|Default|GetDeltaTime) (Variables|Default|GetFadeRate)))))))
      (for _array_element (Variables|Default|GetFadeMatMID)
        (Rendering|Material|SetScalarParameterValue _array_element "opacity" (Math|Curves|GetFloatValue (Variables|Default|GetfadeCurve) (Variables|Default|GetCurrentFade)) :!class /Script/Engine.MaterialInstanceDynamic)))))

(fn ToggleHideMesh
  (params (Hidden :type Boolean))
  (if (Math|Boolean|NotEqual(Boolean) Hidden (Variables|Default|GetHidden))
    (Variables|Default|SetHidden Hidden)))