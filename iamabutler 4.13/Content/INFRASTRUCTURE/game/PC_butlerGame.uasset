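; Player controller for the butler game that owns the in-game HUD and escape menu.
; On BeginPlay outside the main menu level, it creates the test UI widget on screen and prepares the escape menu.
; Escape toggles that menu, H tells the HUD to show controls, and an adjustHappiness event subtracts the passed amount from the HUD's happiness value.
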(event Custom|adjustHappiness
  (params (happinessAdjustment :type Float%20%28single-precision%29))
  (bind _playerui (Variables|Default|GetplayerUI))
  (Variables|/Game/INFRASTRUCTURE/UMG/W_testUI.W_testUI_C|SethappinessValue _playerui (- (Variables|/Game/INFRASTRUCTURE/UMG/W_testUI.W_testUI_C|GethappinessValue _playerui) (/ happinessAdjustment 1.0))))

(event EventBeginPlay
  (bind _returnvalue (Game|GetCurrentLevelName true))
  (if (not (Utilities|Enum|Equal(Enum) _returnvalue "mainMenu"))
    (bind _returnvalue_2 (UserInterface|CreateWidget "/Game/INFRASTRUCTURE/UMG/W_testUI.W_testUI_C"))
    (bind _output_get (Variables|Default|SetplayerUI _returnvalue_2))
    (UserInterface|Viewport|AddtoViewport _output_get 0)
    (bind _returnvalue_3 (UserInterface|CreateWidget "/Game/INFRASTRUCTURE/UMG/W_escapeMenu.W_escapeMenu_C"))
    (Variables|Default|SetescMenu _returnvalue_3)))

(event EventTick
  (params (DeltaSeconds :type Float%20%28single-precision%29)))

(event Input|KeyboardEvents|Escape
  (params (Key :type Key%20Structure :default "AnyKey"))
  (bind _escmenu (Variables|Default|GetescMenu))
  (:Pressed
    (if (UserInterface|Viewport|IsinViewport _escmenu)
      (Default|Remove _escmenu)
      (else
        (UserInterface|Viewport|AddtoViewport _escmenu 0)))))

(event Input|KeyboardEvents|H
  (params (Key :type Key%20Structure :default "AnyKey"))
  (:Pressed
    (Default|ShowControls (Variables|Default|GetplayerUI))))

(fn ConstructionScript)