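; Spawner actor that scatters random breakable objects inside a box extent, starting on BeginPlay when AutoStart is set or via startSpawning.
; A looping timer, its period a random interval divided by the object total, picks a random BP_breakableMaster class from a list and spawns it with effect and sound.
; Each object gets random linear and angular impulses.
; The timer clears once the spawned count exceeds the total.
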(event Custom|startSpawning
  (bind _returnvalue (Utilities|Time|SetTimerbyFunctionName 0 "spawnObject" (/ (Math|Random|RandomFloatinRange (Variables|Default|GetintervalMin) (Variables|Default|GetintervalMax)) (Math|Conversions|ToFloat(Integer) (Variables|Default|GettotalObjectsToSpawn))) true))
  (Variables|Default|SetspawnObject_timer _returnvalue))

(event Custom|spawnObject
  (bind _returnvalue (Math|Random|RandomFloatinRange -5.0 5.0))
  (bind _spawnextent (Variables|Default|GetSpawnExtent))
  (CallFunction|RandomizeSpawnedObject)
  (bind _output_get (Variables|Default|SetspawnLoc (Math|Random|RandomPointinBoundingBox (Transformation|GetWorldLocation _spawnextent) (Components|Box|GetScaledBoxExtent _spawnextent))))
  (Effects|SpawnEmitteratLocation "/Game/ASSETS/particles/P_spawn.P_spawn" _output_get)
  (Audio|PlaySoundatLocation "/Game/ASSETS/sounds/SC_objectSpawned.SC_objectSpawned" _output_get)
  (bind _returnvalue_2 (Game|SpawnActorfromClass (Variables|Default|GetbreakableObjectClass) (Math|Transform|MakeTransform _output_get "0, 0, 0" "1,1,1") "Undefined" 0 "/Game/ASSETS/sounds/SC_objectBreak.SC_objectBreak" 0))
  (Physics|AddImpulse (Variables|/Game/INFRASTRUCTURE/breakables/BP_breakableMaster.BP_breakableMaster_C|GetSM_displayObject _returnvalue_2) (Math|Vector|MakeVector (Math|Random|RandomFloatinRange -5e+01 5e+01) (Math|Random|RandomFloatinRange -5e+01 5e+01) (Math|Random|RandomFloatinRange 25.0 5e+01)) "None" true)
  (Class|PrimitiveComponent|AddAngularImpulse (Variables|/Game/INFRASTRUCTURE/breakables/BP_breakableMaster.BP_breakableMaster_C|GetSM_displayObject _returnvalue_2) (Math|Vector|MakeVector _returnvalue _returnvalue _returnvalue) "None" true)
  (Variables|Default|SetspawnedObjects (+ (Variables|Default|GetspawnedObjects) 1))
  (if (> (Variables|Default|GetspawnedObjects) (Variables|Default|GettotalObjectsToSpawn))
    (Utilities|Time|ClearandInvalidateTimerbyHandle (Variables|Default|GetspawnObject_timer))))

(event EventBeginPlay
  (if (Variables|Default|GetbAutoStart)
    (bind _returnvalue (Utilities|Time|SetTimerbyFunctionName 0 "spawnObject" (/ (Math|Random|RandomFloatinRange (Variables|Default|GetintervalMin) (Variables|Default|GetintervalMax)) (Math|Conversions|ToFloat(Integer) (Variables|Default|GettotalObjectsToSpawn))) true))
    (Variables|Default|SetspawnObject_timer _returnvalue)))

(fn ConstructionScript)

(fn RandomizeSpawnedObject
  (bind _possiblebreakablespawninglist (Variables|Default|GetpossibleBreakableSpawningList))
  (Variables|Default|SetbreakableObjectClass (.AsBP%20Breakable%20Master (Utilities|Casting|CastToBP_breakableMasterClass (Utilities|Array|Get(acopy) _possiblebreakablespawninglist (Math|Random|RandomIntegerinRange 0 (- (Utilities|Array|Length _possiblebreakablespawninglist) 1)))))))